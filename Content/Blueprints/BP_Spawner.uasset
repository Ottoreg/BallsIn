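; BP_Spawner places a local player's ThirdPersonCharacter at the spawner's transform on BeginPlay and assigns its team.
; It decrements PlayerID, then uses the existing first player's pawn if the result is zero, or creates an additional local player otherwise.
; The team comes from the parity of the decremented ID, so players alternate between two teams, and SetTeamColor applies the matching color.
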(event EventBeginPlay
  (Math|Integer|DecrementInt (Variables|Default|GetplayerID)
    (:%20%20
      (if (== 0 (Variables|Default|GetplayerID))
        (bind _asthird_person_character (Utilities|Casting|CastToThirdPersonCharacter (Game|Player|GetPlayerPawn 0)))
        (Variables|/Game/Blueprints/ThirdPersonCharacter.ThirdPersonCharacter_C|Setteam _asthird_person_character (Math|Integer|%(Integer) (Variables|Default|GetplayerID) 2))
        (Default|SetTeamColor _asthird_person_character)
        (Transformation|SetActorTransform _asthird_person_character (Transformation|GetActorTransform))
        (else
          (bind _returnvalue (Class|GameplayStatics|CreatePlayer -1))
          (bind _asthird_person_character_2 (Utilities|Casting|CastToThirdPersonCharacter (Pawn|GetControlledPawn _returnvalue)))
          (Variables|/Game/Blueprints/ThirdPersonCharacter.ThirdPersonCharacter_C|Setteam _asthird_person_character_2 (Math|Integer|%(Integer) (Variables|Default|GetplayerID) 2))
          (Default|SetTeamColor _asthird_person_character_2)
          (Transformation|SetActorTransform _asthird_person_character_2 (Transformation|GetActorTransform)))))))

(fn ConstructionScript)